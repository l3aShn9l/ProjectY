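; BP_GravityCube is a cube whose colour decides the gravity-like force acting on it.
; Every tick it applies a mass-scaled force by colour: Blue pushes down, Red pushes up, and White applies zero force.
; Set events switch colour and material together.
; AddBlue and AddRed shift the cube toward that colour, with opposite colours cancelling to White.
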(event Custom|SetBlue
  (Variables|Default|SetColour "NewEnumerator0")
  (Rendering|Material|SetMaterial (Variables|Default|GetCube) 0 "/Game/ProjectY/Materials/BlueMaterial.BlueMaterial"))

(event Custom|SetRed
  (Variables|Default|SetColour "NewEnumerator2")
  (Rendering|Material|SetMaterial (Variables|Default|GetCube) 0 "/Game/ProjectY/Materials/RedMaterial.RedMaterial"))

(event Custom|SetWhite
  (Variables|Default|SetColour "NewEnumerator1")
  (Rendering|Material|SetMaterial (Variables|Default|GetCube) 0 "/Game/ProjectY/Materials/WhiteMaterial.WhiteMaterial"))

(event EventBeginPlay)

(event Collision|EventActorBeginOverlap
  (params (OtherActor :type Actor%20Object%20Reference)))

(event EventAddRed
  (bind _newparam (CallFunction|GetColour))
  (switch Utilities|FlowControl|Switch|SwitchonE_Colour _newparam
    (:NewEnumerator1
      (CallFunction|SetRed :!label _label))
    (:NewEnumerator0
      (CallFunction|SetWhite))
    (:NewEnumerator2
      (goto _label))))

(event EventTick
  (params (DeltaSeconds :type Float%20%28single-precision%29))
  (bind _newparam (CallFunction|GetColour))
  (switch Utilities|FlowControl|Switch|SwitchonE_Colour _newparam
    (:NewEnumerator1
      (Physics|AddForce (Variables|Default|GetCube) (* (Math|Vector|MakeVector 0.0 0.0 0.0) (Physics|GetMass (Variables|Default|GetCube))) "None" false))
    (:NewEnumerator0
      (Physics|AddForce (Variables|Default|GetCube) (* (Math|Vector|MakeVector 0.0 0.0 -9.8e+02) (Physics|GetMass (Variables|Default|GetCube))) "None" false))
    (:NewEnumerator2
      (Physics|AddForce (Variables|Default|GetCube) (* (Math|Vector|MakeVector 0.0 0.0 9.8e+02) (Physics|GetMass (Variables|Default|GetCube))) "None" false))))

(event EventAddBlue
  (bind _newparam (CallFunction|GetColour))
  (switch Utilities|FlowControl|Switch|SwitchonE_Colour _newparam
    (:NewEnumerator1
      (CallFunction|SetBlue :!label _label))
    (:NewEnumerator0
      (goto _label))
    (:NewEnumerator2
      (CallFunction|SetWhite))))

(fn ConstructionScript)

(fn GetColour
  (return (Variables|Default|GetColour)))