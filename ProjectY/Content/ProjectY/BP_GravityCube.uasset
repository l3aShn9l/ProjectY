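; BP_GravityCube is a cube actor whose vertical pull depends on its colour state.
; Each Tick it reads Colour and applies a mass-scaled force to the Cube: downward for Blue, none for White, upward for Red.
; SetBlue, SetRed and SetWhite events switch the state, and scaling by mass gives a gravity-like acceleration whatever the cube weighs.
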(event EventBeginPlay)

(event Collision|EventActorBeginOverlap
  (params (OtherActor :type Actor%20Object%20Reference)))

(event EventTick
  (params (DeltaSeconds :type Float%20%28single-precision%29))
  (bind _newparam (CallFunction|GetColour))
  (switch Utilities|FlowControl|Switch|SwitchonE_Colour _newparam
    (:NewEnumerator0
      (Physics|AddForce (Variables|Default|GetCube) (* (Math|Vector|MakeVector 0.0 0.0 -9.8e+02) (Physics|GetMass (Variables|Default|GetCube))) "None" false))
    (:NewEnumerator1
      (Physics|AddForce (Variables|Default|GetCube) (* (Math|Vector|MakeVector 0.0 0.0 0.0) (Physics|GetMass (Variables|Default|GetCube))) "None" false))
    (:NewEnumerator2
      (Physics|AddForce (Variables|Default|GetCube) (* (Math|Vector|MakeVector 0.0 0.0 9.8e+02) (Physics|GetMass (Variables|Default|GetCube))) "None" false))))

(event EventSetBlue
  (Variables|Default|SetColour "NewEnumerator0"))

(event EventSetRed
  (Variables|Default|SetColour "NewEnumerator2"))

(event EventSetWhite
  (Variables|Default|SetColour "NewEnumerator1"))

(fn ConstructionScript)

(fn GetColour
  (return (Variables|Default|GetColour)))